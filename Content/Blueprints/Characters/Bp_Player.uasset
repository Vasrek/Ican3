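; Player character Blueprint that handles movement, camera look, jumping, checkpoint respawning, coin and death tracking, and the win state.
; BeginPlay stores the start transform and creates the HUD; checkpoints update that transform, and death teleports back to it and updates the HUD counter.
; A pause toggle creates or removes the in-game menu, switching pause, input and cursor, and syncing the menu reference to PC_Level1.
; Winning notifies listeners, locks input and hides the HUD.
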(event Custom|Death
  ;[1 1 1] Teleport the player on the correct checkpoint transform
  (Transformation|SetActorTransform (Variables|Character|GetRespawnTransform) false true)
  (bind _result (Math|Integer|IncrementInt (Variables|Widget|GetDeathCounter))
    (:%20%20
      (Default|UpdateDeathCounter (Variables|Widget|GetHUD_Ref) _result))))

(event Custom|Checkpoint
  (params (RespawnTransform :type Transform))
  ;[1 1 1] Set new checkpoint transform
  (Variables|Character|SetRespawnTransform RespawnTransform))

(event Custom|Win
  (bind _returnvalue (Game|GetPlayerController 0))
  ;[1 1 1] Win - disable player movement and camera input - hide hud ref
  (Default|CallPlayerHasWon)
  (Input|SetIgnoreLookInput _returnvalue true)
  (Input|SetIgnoreMoveInput _returnvalue true)
  (Widget|SetVisibility (Variables|Widget|GetHUD_Ref) "Hidden"))

(event Custom|AddCoin
  (params (CoinToAdd :type Integer))
  ;[1 1 1] Increase coin + update it from widget
  (bind _output_get (Variables|Widget|SetCoins (+ CoinToAdd (Variables|Widget|GetCoins))))
  (Default|UpdateGoldCounter (Variables|Widget|GetHUD_Ref) _output_get))

(event Custom|RemoveInGamePauseMenu
  (bind _returnvalue (Game|GetPlayerController 0))
  (bind _returnvalue_2 (Game|GetPlayerController 0))
  (bind _pcref (Variables|Default|GetPCRef))
  ;[1 1 1] Pause menu - if the widget is already displayeed -> removed it; if the widget do not exist -> display it (enable or disable movement input + camera and set game paused
  (Utilities|IsValid (Variables|Widget|GetIngamePauseMenuRef)
    (:Is%20Valid
      (Widget|RemovefromParent (Variables|Widget|GetIngamePauseMenuRef))
      (Input|SetIgnoreLookInput _returnvalue false)
      (Input|SetIgnoreMoveInput _returnvalue false)
      (Game|SetGamePaused false)
      (Variables|/Script/Engine.PlayerController|SetbShowMouseCursor _returnvalue false)
      (Input|SetInputModeGameOnly _returnvalue)
      (Variables|Widget|SetIngamePauseMenuRef 0)
      (Variables|/Game/Blueprints/Core/PC_Level1.PC_Level1_C|SetInGameMenuRef _pcref 0)
      (Variables|/Game/Blueprints/Core/PC_Level1.PC_Level1_C|SetVIndex _pcref 0))
    (:Is%20Not%20Valid
      (bind _returnvalue_3 (UserInterface|CreateWidget "/Game/Blueprints/Widgets/WBP_InGamePauseMenu.WBP_InGamePauseMenu_C"))
      (bind _output_get (Variables|Widget|SetIngamePauseMenuRef _returnvalue_3))
      (UserInterface|Viewport|AddtoViewport _output_get 0)
      (Game|SetGamePaused true)
      (Input|SetIgnoreMoveInput _returnvalue_2 true)
      (Input|SetIgnoreLookInput _returnvalue_2 true)
      (Variables|/Script/Engine.PlayerController|SetbShowMouseCursor _returnvalue_2 true)
      (Input|SetInputModeGameandUI _returnvalue_2 (Variables|Widget|GetIngamePauseMenuRef) "DoNotLock" false)
      (Variables|/Game/Blueprints/Core/PC_Level1.PC_Level1_C|SetInGameMenuRef _pcref (Variables|Widget|GetIngamePauseMenuRef))
      (Default|HoverControllerResume (Variables|Widget|GetIngamePauseMenuRef)))))

(event EventBeginPlay
  (bind _returnvalue (Game|GetPlayerController 0))
  ;[1 1 1] Enable movement input + display hud widget
  (Variables|Character|SetRespawnTransform (Transformation|GetActorTransform))
  (bind _returnvalue_2 (UserInterface|CreateWidget "/Game/Blueprints/Widgets/WBP_Hud.WBP_Hud_C"))
  (bind _output_get (Variables|Widget|SetHUD_Ref _returnvalue_2))
  (UserInterface|Viewport|AddtoViewport _output_get 0)
  (Variables|/Script/Engine.PlayerController|SetbShowMouseCursor _returnvalue false)
  (Input|SetInputModeGameOnly _returnvalue)
  (bind _aspc_level_1 (Utilities|Casting|CastToPC_Level1 _returnvalue))
  (Variables|Default|SetPCRef _aspc_level_1))

(event Input|ActionEvents|InputActionJump
  (params (Key :type Key%20Structure :default "None"))
  ;[0.1423 1 0.3342] Input
  (:Pressed
    (Character|Jump))
  (:Released
    (Character|StopJumping)))

(event Input|ActionEvents|InputActionIngamePauseMenu
  (params (Key :type Key%20Structure :default "None"))
  (bind _returnvalue (Game|GetPlayerController 0))
  (bind _returnvalue_2 (Game|GetPlayerController 0))
  (bind _pcref (Variables|Default|GetPCRef))
  ;[1 1 1] Pause menu - if the widget is already displayeed -> removed it; if the widget do not exist -> display it (enable or disable movement input + camera and set game paused
  (:Pressed
    (Utilities|IsValid (Variables|Widget|GetIngamePauseMenuRef)
      (:Is%20Valid
        (Widget|RemovefromParent (Variables|Widget|GetIngamePauseMenuRef))
        (Input|SetIgnoreLookInput _returnvalue false)
        (Input|SetIgnoreMoveInput _returnvalue false)
        (Game|SetGamePaused false)
        (Variables|/Script/Engine.PlayerController|SetbShowMouseCursor _returnvalue false)
        (Input|SetInputModeGameOnly _returnvalue)
        (Variables|Widget|SetIngamePauseMenuRef 0)
        (Variables|/Game/Blueprints/Core/PC_Level1.PC_Level1_C|SetInGameMenuRef _pcref 0)
        (Variables|/Game/Blueprints/Core/PC_Level1.PC_Level1_C|SetVIndex _pcref 0))
      (:Is%20Not%20Valid
        (bind _returnvalue_3 (UserInterface|CreateWidget "/Game/Blueprints/Widgets/WBP_InGamePauseMenu.WBP_InGamePauseMenu_C"))
        (bind _output_get (Variables|Widget|SetIngamePauseMenuRef _returnvalue_3))
        (UserInterface|Viewport|AddtoViewport _output_get 0)
        (Game|SetGamePaused true)
        (Input|SetIgnoreMoveInput _returnvalue_2 true)
        (Input|SetIgnoreLookInput _returnvalue_2 true)
        (Variables|/Script/Engine.PlayerController|SetbShowMouseCursor _returnvalue_2 true)
        (Input|SetInputModeGameandUI _returnvalue_2 (Variables|Widget|GetIngamePauseMenuRef) "DoNotLock" false)
        (Variables|/Game/Blueprints/Core/PC_Level1.PC_Level1_C|SetInGameMenuRef _pcref (Variables|Widget|GetIngamePauseMenuRef))
        (Default|HoverControllerResume (Variables|Widget|GetIngamePauseMenuRef))))))

(event Input|AxisEvents|InputAxisMoveForwardBackward
  (params (AxisValue :type Float%20%28single-precision%29))
  ;[0.1423 1 0.3342] Input
  (Pawn|Input|AddMovementInput (Math|Vector|GetForwardVector (Math|Rotator|MakeRotator 0.0 0.0 (.yaw (Pawn|GetControlRotation :!class /Script/Engine.Pawn)))) AxisValue false))

(event Input|AxisEvents|InputAxisMoveLeftRight
  (params (AxisValue :type Float%20%28single-precision%29))
  ;[0.1423 1 0.3342] Input
  (Pawn|Input|AddMovementInput (Math|Vector|GetRightVector (Math|Rotator|MakeRotator 0.0 0.0 (.yaw (Pawn|GetControlRotation :!class /Script/Engine.Pawn)))) AxisValue false))

(event Input|AxisEvents|InputAxisLook
  (params (AxisValue :type Float%20%28single-precision%29))
  ;[0.1423 1 0.3342] Input
  (Pawn|Input|AddControllerYawInput AxisValue))

(event Input|AxisEvents|InputAxisLookUp
  (params (AxisValue :type Float%20%28single-precision%29))
  ;[0.1423 1 0.3342] Input
  (Pawn|Input|AddControllerPitchInput AxisValue))

(fn ConstructionScript)