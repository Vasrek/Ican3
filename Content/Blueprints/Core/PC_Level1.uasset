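; PC_Level1 is the Level 1 player controller that adds gamepad navigation to the in-game menu.
; D-pad up and down step a clamped VIndex, then clear all button highlights and hover Resume, Main Menu or Quit on InGameMenuRef.
; The bottom face button fires the click handler for the selected index.
; All input is ignored unless the menu reference is valid, and this file never assigns that reference.
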(event Input|GamepadEvents|GamepadDPadDown
  (params (Key :type Key%20Structure :default "None"))
  (bind _ingamemenuref (Variables|Default|GetInGameMenuRef))
  (:Pressed
    (Utilities|IsValid (Variables|Default|GetInGameMenuRef)
      (:Is%20Valid
        (bind _result (Math|Integer|IncrementInt (Variables|Default|GetVIndex))
          (:%20%20
            (if (>= _result (Variables|Default|GetMaxVIndex))
              (Variables|Default|SetVIndex (Variables|Default|GetMaxVIndex)))
            (Default|UnhoverAllButtons (Variables|Default|GetInGameMenuRef))
            (switch int (Variables|Default|GetVIndex)
              (:0
                (Default|HoverControllerResume _ingamemenuref))
              (:1
                (Default|HoverControllerMainMenu _ingamemenuref))
              (:2
                (Default|HoverControllerQuit _ingamemenuref)))))))))

(event Input|GamepadEvents|GamepadDPadUp
  (params (Key :type Key%20Structure :default "None"))
  (bind _ingamemenuref (Variables|Default|GetInGameMenuRef))
  (:Pressed
    (Utilities|IsValid (Variables|Default|GetInGameMenuRef)
      (:Is%20Valid
        (bind _result (Math|Integer|DecrementInt (Variables|Default|GetVIndex))
          (:%20%20
            (if (<= _result 0)
              (Variables|Default|SetVIndex 0))
            (Default|UnhoverAllButtons (Variables|Default|GetInGameMenuRef))
            (switch int (Variables|Default|GetVIndex)
              (:0
                (Default|HoverControllerResume _ingamemenuref))
              (:1
                (Default|HoverControllerMainMenu _ingamemenuref))
              (:2
                (Default|HoverControllerQuit _ingamemenuref)))))))))

(event Input|GamepadEvents|GamepadFaceButtonBottom
  (params (Key :type Key%20Structure :default "None"))
  (bind _ingamemenuref (Variables|Default|GetInGameMenuRef))
  (:Pressed
    (Utilities|IsValid (Variables|Default|GetInGameMenuRef)
      (:Is%20Valid
        (switch int (Variables|Default|GetVIndex)
          (:0
            (Default|ClickedControllerResume _ingamemenuref))
          (:1
            (Default|ClickedControllerMainMenu _ingamemenuref))
          (:2
            (Default|ClickedControllerQuit _ingamemenuref)))))))

(fn ConstructionScript)