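; Player controller for the main menu that creates the menu widget and adds gamepad navigation for its Play and Quit buttons.
; On BeginPlay it adds WBP_MainMenu to the viewport and sets Game and UI input mode focused on it.
; D-pad Up and Down move a clamped index, which clears all hovers and highlights the selected button.
; The bottom face button triggers that button's click handler on the widget.
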(event EventBeginPlay
  ;[1 1 1] Create widget main menu + set input mode ui and game only
  (bind _returnvalue (UserInterface|CreateWidget "/Game/Blueprints/Widgets/WBP_MainMenu.WBP_MainMenu_C"))
  (bind _output_get (Variables|Default|SetMainMenuRef _returnvalue))
  (UserInterface|Viewport|AddtoViewport _output_get 0)
  (Input|SetInputModeGameandUI (Game|GetPlayerController 0) (Variables|Default|GetMainMenuRef) "DoNotLock" true))

(event Input|GamepadEvents|GamepadDPadDown
  (params (Key :type Key%20Structure :default "None"))
  (bind _mainmenuref (Variables|Default|GetMainMenuRef))
  ;[1 1 1] Xbox controller è Up/Down hover/unhover main menu buttons
  (:Pressed
    (if (>= (Variables|Default|GetVIndex_MainMenu) 1)
      (Variables|Default|SetVIndex_MainMenu 1)
      (else
        (Math|Integer|IncrementInt (Variables|Default|GetVIndex_MainMenu)
          (:%20%20
            _))))
    (Default|UnHoverAllButtonsController _mainmenuref)
    (switch int (Variables|Default|GetVIndex_MainMenu)
      (:0
        (Default|HoverPlayController _mainmenuref))
      (:1
        (Default|HoverQuitController _mainmenuref)))))

(event Input|GamepadEvents|GamepadDPadUp
  (params (Key :type Key%20Structure :default "None"))
  (bind _mainmenuref (Variables|Default|GetMainMenuRef))
  ;[1 1 1] Xbox controller è Up/Down hover/unhover main menu buttons
  (:Pressed
    (if (<= (Variables|Default|GetVIndex_MainMenu) 0)
      (Variables|Default|SetVIndex_MainMenu 0)
      (else
        (Math|Integer|DecrementInt (Variables|Default|GetVIndex_MainMenu)
          (:%20%20
            _))))
    (Default|UnHoverAllButtonsController _mainmenuref)
    (switch int (Variables|Default|GetVIndex_MainMenu)
      (:0
        (Default|HoverPlayController _mainmenuref))
      (:1
        (Default|HoverQuitController _mainmenuref)))))

(event Input|GamepadEvents|GamepadFaceButtonBottom
  (params (Key :type Key%20Structure :default "None"))
  (bind _mainmenuref (Variables|Default|GetMainMenuRef))
  ;[1 1 1] GamepadController - Click Play/Quit
  (:Pressed
    (switch int (Variables|Default|GetVIndex_MainMenu)
      (:0
        (Default|OnClickedPlayController _mainmenuref))
      (:1
        (Default|OnClickedQuitController _mainmenuref)))))

(fn ConstructionScript)