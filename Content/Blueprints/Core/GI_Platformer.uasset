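; Game instance for the platformer that persists the player's best score to a save slot.
; SaveScore loads the existing SG_ScorePlayer save and overwrites BestScore only when the new score equals or beats it.
; If no save exists, it creates one with the submitted score and writes it to the slot.
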(event Custom|SaveScore
  (params (ScoreToCheck :type Integer))
  (bind _returnvalue (SaveGame|DoesSaveGameExist (Variables|Default|GetSaveGameSlot)))
  (if _returnvalue
    (bind _returnvalue_2 (SaveGame|LoadGamefromSlot (Variables|Default|GetSaveGameSlot)))
    (bind _assg_score_player (Utilities|Casting|CastToSG_ScorePlayer _returnvalue_2))
    (Variables|Default|SetSaveGameObject _assg_score_player)
    (if (>= ScoreToCheck (Variables|/Game/Blueprints/Core/SG_ScorePlayer.SG_ScorePlayer_C|GetBestScore _assg_score_player))
      (Variables|/Game/Blueprints/Core/SG_ScorePlayer.SG_ScorePlayer_C|SetBestScore _assg_score_player ScoreToCheck)
      (SaveGame|SaveGametoSlot (Variables|Default|GetSaveGameObject) (Variables|Default|GetSaveGameSlot) :!label _label))
    (else
      (bind _returnvalue_3 (SaveGame|CreateSaveGameObject "/Game/Blueprints/Core/SG_ScorePlayer.SG_ScorePlayer_C"))
      (Variables|/Game/Blueprints/Core/SG_ScorePlayer.SG_ScorePlayer_C|SetBestScore _returnvalue_3 ScoreToCheck)
      (Variables|Default|SetSaveGameObject _returnvalue_3)
      (goto _label))))