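; BP_FakePlatform is a two-sided platform actor where one randomly chosen side is fake and falls away.
; On BeginPlay, a coin flip sets LeftFake to pick the left or right cube.
; Bp_Player overlapping either trigger box runs shared logic that drops the fake cube, whichever box was touched.
; The cube falls by enabling physics simulation, then is destroyed after a short delay.
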(event OnComponentBeginOverlap(BoxLeft)
  (params (OverlappedComponent :type Primitive%20Component%20Object%20Reference) (OtherActor :type Actor%20Object%20Reference) (OtherComp :type Primitive%20Component%20Object%20Reference) (OtherBodyIndex :type Integer) (bFromSweep :type Boolean) (SweepResult :type Hit%20Result%20Structure%20%28by%20ref%29))
  (Variables|Default|SetOther%20Actor OtherActor)
  (Utilities|Casting|CastToBp_Player (Variables|Default|GetOther%20Actor))
  (if (Variables|Default|GetLeftFake?)
    (Variables|Default|SetPlatformToFall (Variables|Default|GetCubeLelft))
    (else
      (Variables|Default|SetPlatformToFall (Variables|Default|GetCubeRight))))
  (Utilities|IsValid (Variables|Default|GetPlatformToFall)
    (:Is%20Valid
      (Physics|SetSimulatePhysics (Variables|Default|GetPlatformToFall) true)
      (Utilities|FlowControl|Delay 5.0)
      (Components|DestroyComponent (Variables|Default|GetPlatformToFall)))))

(event OnComponentBeginOverlap(BoxRight)
  (params (OverlappedComponent :type Primitive%20Component%20Object%20Reference) (OtherActor :type Actor%20Object%20Reference) (OtherComp :type Primitive%20Component%20Object%20Reference) (OtherBodyIndex :type Integer) (bFromSweep :type Boolean) (SweepResult :type Hit%20Result%20Structure%20%28by%20ref%29))
  (Variables|Default|SetOther%20Actor OtherActor)
  (Utilities|Casting|CastToBp_Player (Variables|Default|GetOther%20Actor))
  (if (Variables|Default|GetLeftFake?)
    (Variables|Default|SetPlatformToFall (Variables|Default|GetCubeLelft))
    (else
      (Variables|Default|SetPlatformToFall (Variables|Default|GetCubeRight))))
  (Utilities|IsValid (Variables|Default|GetPlatformToFall)
    (:Is%20Valid
      (Physics|SetSimulatePhysics (Variables|Default|GetPlatformToFall) true)
      (Utilities|FlowControl|Delay 5.0)
      (Components|DestroyComponent (Variables|Default|GetPlatformToFall)))))

(event EventBeginPlay
  (if (== (Math|Random|RandomIntegerinRange 0 1) 0)
    (Variables|Default|SetLeftFake? true)
    (else
      (Variables|Default|SetLeftFake? false))))

(fn ConstructionScript)