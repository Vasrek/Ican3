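; BP_FallingPlatform is a platform that drops shortly after the player steps into its trigger box, then returns to its start position.
; On overlap with Bp_Player, delays time the switch to physics simulation on the Cube and the later reset.
; The reset disables physics and teleports the Cube to the transform cached at BeginPlay.
; The construction script gives the Cube a random color from seven material instances.
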(event OnComponentBeginOverlap(Box)
  (params (OverlappedComponent :type Primitive%20Component%20Object%20Reference) (OtherActor :type Actor%20Object%20Reference) (OtherComp :type Primitive%20Component%20Object%20Reference) (OtherBodyIndex :type Integer) (bFromSweep :type Boolean) (SweepResult :type Hit%20Result%20Structure%20%28by%20ref%29))
  (Utilities|Casting|CastToBp_Player OtherActor)
  (Utilities|FlowControl|Delay 1.0)
  (Physics|SetSimulatePhysics (Variables|Default|GetCube) true)
  (Utilities|FlowControl|Delay 5.0)
  (Physics|SetSimulatePhysics (Variables|Default|GetCube) false)
  (Transformation|SetWorldTransform (Variables|Default|GetCube) (Variables|Default|GetDefautLoc) false true))

(event EventBeginPlay
  (Variables|Default|SetDefautLoc (Transformation|GetWorldTransform (Variables|Default|GetCube))))

(fn ConstructionScript
  (Rendering|Material|SetMaterial (Variables|Default|GetCube) 0 (Utilities|Select :Index (Math|Random|RandomIntegerinRange 0 6) :Option%200 "/Game/Materials/M_BlueInst.M_BlueInst" :Option%201 "/Game/Materials/M_BrownInst.M_BrownInst" :Option%202 "/Game/Materials/M_Greennst.M_Greennst" :Option%203 "/Game/Materials/M_PinkInst.M_PinkInst" :Option%204 "/Game/Materials/M_PurpleInst.M_PurpleInst" :Option%205 "/Game/Materials/M_RedInst.M_RedInst" :Option%206 "/Game/Materials/M_YellowInst.M_YellowInst")))